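; BP_CheckPoint is a checkpoint actor that moves the player's spawn point when a player passes through it.
; Its Sphere overlap accepts only BP_Players and writes the CheckTransform component's world transform into GM_InGame's SpawnTransform.
; An equality check skips the update when this checkpoint is already the active spawn, so the enlarged explosion effect near the actor plays only when the spawn point changes.
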(event `self.Sphere.OnComponentBeginOverlap`
  (params (OverlappedComponent :type "PrimitiveComponent Object Reference") (OtherActor :type "Actor Object Reference") (OtherComp :type "PrimitiveComponent Object Reference") (OtherBodyIndex :type Integer) (bFromSweep :type Boolean) (SweepResult :type "HitResult Structure (by ref)"))
  (bind _returnvalue (`SceneComponent.K2_GetComponentToWorld` (`self.CheckTransform`)))
  ;[1 1 1] Playerが通過したらSpawnTransformを変更する
  (cast `/Game/MyContens/BluePrint/BP_Players` OtherActor)
  (bind _asgm_in_game (cast `/Game/MyContens/GM_InGame` (`GameplayStatics.GetGameMode`)))
  (if (not (== (`/Game/MyContens/GM_InGame.SpawnTransform` _asgm_in_game) _returnvalue))
    (set `/Game/MyContens/GM_InGame.SpawnTransform` _returnvalue _asgm_in_game)
    (`GameplayStatics.SpawnEmitterAtLocation` "/Game/StarterContent/Particles/P_Explosion.P_Explosion" (+ (0.0 -100.0 100.0) (`self.K2_GetActorLocation`)) (struct) (5.0 5.0 5.0))))

(fn `UserConstructionScript`)