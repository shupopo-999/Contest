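; Player blueprint for a physics-driven mesh, SMPlayer, controlled through Enhanced Input with the IM_Control mapping context.
; Movement applies force relative to the Arrow component's transform, while look input turns the controller and zeroes its roll.
; Jump applies an upward impulse, locked until any Hit event re-enables it.
; Boost and Slow apply torque derived from the arrow's forward vector, with Slow dividing where Boost multiplies.
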(event `self.ReceiveBeginPlay`
  (bind _returnvalue (pcsubsystem `EnhancedInputLocalPlayerSubsystem` (`GameplayStatics.GetPlayerController` 0)))
  ;[1 1 1] InputをIM_Controlに設定
  (`/Engine/EditorBlueprintResources/StandardMacros.IsValid` _returnvalue
    (:`Is Valid`
      (`EnhancedInputSubsystemInterface.AddMappingContext` _returnvalue "/Game/MyContens/IM_Control.IM_Control" 0 (struct)))))

(event `EnhancedInput|/Game/MyContens/InputAction/IA_Control`
  (params (ActionValue :type "Vector2D Structure") (ElapsedSeconds :type "Float (double-precision)") (TriggeredSeconds :type "Float (double-precision)") (InputAction :type "InputAction Object Reference" :default "/Game/MyContens/InputAction/IA_Control.IA_Control"))
  (bind (_x _y) (`KismetMathLibrary.BreakVector2D` ActionValue))
  ;[1 1 1] 力を加える設定
  (:`Triggered`
    (`PrimitiveComponent.AddForce` (`self.SM_Player`) (* (`KismetMathLibrary.TransformDirection` (`SceneComponent.K2_GetComponentToWorld` (`self.Arrow`)) (`KismetMathLibrary.MakeVector` _y _x)) (`self.Speed`)) "None" true)))

(event `EnhancedInput|/Game/MyContens/InputAction/IA_Look`
  (params (ActionValue :type "Vector2D Structure") (ElapsedSeconds :type "Float (double-precision)") (TriggeredSeconds :type "Float (double-precision)") (InputAction :type "InputAction Object Reference" :default "/Game/MyContens/InputAction/IA_Look.IA_Look"))
  (bind (_x _y) (`KismetMathLibrary.BreakVector2D` ActionValue))
  ;[1 1 1] コントローラーの角度を変更する
  (:`Triggered`
    (`|ExecutionSequence`
      (:`then_0`
        (`self.AddControllerYawInput` _x)
        (`self.AddControllerPitchInput` _y))
      (:`then_1`
        ;[1 1 1] カメラの操作を制限する
        (`Controller.SetControlRotation` (`GameplayStatics.GetPlayerController` 0) (`KismetMathLibrary.MakeRotator` 0.0 (.pitch (`self.GetControlRotation`)) (.yaw (`self.GetControlRotation`))))))))

(event `EnhancedInput|/Game/ThirdPerson/Input/Actions/IA_Jump`
  (params (ActionValue :type Boolean) (ElapsedSeconds :type "Float (double-precision)") (TriggeredSeconds :type "Float (double-precision)") (InputAction :type "InputAction Object Reference" :default "/Game/ThirdPerson/Input/Actions/IA_Jump.IA_Jump"))
  ;[1 1 1] Playerをジャンプさせる
  (:`Triggered`
    (if (and ActionValue (`self.CamJump`))
      (`PrimitiveComponent.AddImpulse` (`self.SM_Player`) (`KismetMathLibrary.MakeVector` 0.0 0.0 (`self.JumpImpluse`)) "None" true)
      (set `self.CamJump` false))))

(event `self.ReceiveHit`
  (params (MyComp :type "PrimitiveComponent Object Reference") (Other :type "Actor Object Reference") (OtherComp :type "PrimitiveComponent Object Reference") (bSelfMoved :type Boolean) (HitLocation :type "Vector Structure") (HitNormal :type "Vector Structure") (NormalImpulse :type "Vector Structure") (Hit :type "HitResult Structure (by ref)"))
  ;[1 1 1] 再度ジャンプを可能にする
  (set `self.CamJump` true))

(event `EnhancedInput|/Game/MyContens/InputAction/IA_Boost`
  (params (ActionValue :type Boolean) (ElapsedSeconds :type "Float (double-precision)") (TriggeredSeconds :type "Float (double-precision)") (InputAction :type "InputAction Object Reference" :default "/Game/MyContens/InputAction/IA_Boost.IA_Boost"))
  (bind _torque (`self.Torque`))
  ;[1 1 1] Playerを加速させる
  (:`Triggered`
    (if ActionValue
      (`PrimitiveComponent.AddTorqueInRadians` (`self.SM_Player`) (`KismetMathLibrary.MakeVector` (* (.y (`KismetMathLibrary.Normal` (`SceneComponent.GetForwardVector` (`self.Arrow`)))) _torque -1.0) (* (.x (`KismetMathLibrary.Normal` (`SceneComponent.GetForwardVector` (`self.Arrow`)))) _torque)) "None" false))))

(event `EnhancedInput|/Game/MyContens/InputAction/IA_Slow`
  (params (ActionValue :type Boolean) (ElapsedSeconds :type "Float (double-precision)") (TriggeredSeconds :type "Float (double-precision)") (InputAction :type "InputAction Object Reference" :default "/Game/MyContens/InputAction/IA_Slow.IA_Slow"))
  (bind _torque (`self.Torque`))
  ;[1 1 1] Playerを減速させる
  (:`Triggered`
    (if true
      (`PrimitiveComponent.AddTorqueInRadians` (`self.SM_Player`) (`KismetMathLibrary.MakeVector` (/ _torque (.y (`KismetMathLibrary.Normal` (`SceneComponent.GetForwardVector` (`self.Arrow`)))) 1.0) (/ (.x (`KismetMathLibrary.Normal` (`SceneComponent.GetForwardVector` (`self.Arrow`)))) _torque)) "None" false))))

(fn `UserConstructionScript`)